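; Radial menu actor with nested submenus, driven by thumbstick and forwarding trigger input, with motion controller transforms, to the hovered item.
; Data table rows list item actor classes to spawn around a circle; a row named after an item's class marks a submenu, with a history array for going back.
; Stick angle picks the hovered item outside a dead zone, updating focus and a dynamic material.
; Shoulder press selects, or toggles scale-animated show/hide when nothing is hovered.
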(event Custom|FocusMenuItem
  (params (HoverIndex :type Integer))
  (bind _menuitemactors (Variables|Default|GetMenuItemActors))
  (bind _output (Utilities|Array|Get(acopy) _menuitemactors HoverIndex))
  (if (!= HoverIndex -1)
    (if (!= HoverIndex (Variables|Default|GetLastHoverIndex))
      (Utilities|IsValid _output
        (:Is%20Valid
          (Class|BPIMenuItems|Focus(Message) _output))
        (:Is%20Not%20Valid
          _))
      (Utilities|IsValid (Utilities|Array|Get(acopy) (Variables|Default|GetMenuItemActors) (Variables|Default|GetLastHoverIndex))
        (:Is%20Valid
          (Class|BPIMenuItems|Unfocus(Message) (Utilities|Array|Get(acopy) (Variables|Default|GetMenuItemActors) (Variables|Default|GetLastHoverIndex))))
        (:Is%20Not%20Valid
          _))
      (Variables|Default|SetLastHoverIndex HoverIndex))))

(event Custom|Reveal
  (bind _newtrack_0 (Timeline|ScaleActor PlayFromStart)
    (:Update
      (Transformation|SetActorRelativeScale3D self (Math|Conversions|ToVector(Float) _newtrack_0)))))

(event Custom|GoBack
  (bind _menuitemactors (Variables|Default|GetMenuItemActors))
  (bind _datatablerowhistory (Variables|Default|GetDataTableRowHistory))
  (bind _datatablerowhistory_2 (Variables|Default|GetDataTableRowHistory))
  (if (> (Utilities|Array|Length _datatablerowhistory) 1)
    (Utilities|Array|RemoveIndex _datatablerowhistory (Utilities|Array|LastIndex _datatablerowhistory))
    (Utilities|Array|Clear (Variables|Default|GetMenuItemClasses))
    (Variables|Default|SetHoverIndex -1)
    (Variables|Default|SetLastHoverIndex -1)
    (CallFunction|UpdateMaterial (Math|Vector2D|MakeVector2D 0.0 0.0) true)
    (CallFunction|UnfocusMenuItem)
    (for _array_element _menuitemactors
      (Class|BPIMenuItems|FadeOut(Remove)(Message) _array_element))
    (Utilities|Array|Clear _menuitemactors)
    (bind _returnvalue (Utilities|GetDataTableRow (Variables|Default|GetDataTable) (Utilities|Array|Get(acopy) _datatablerowhistory_2 (Utilities|Array|LastIndex _datatablerowhistory_2)))
      (:then
        (bind _output_get (Variables|Default|SetMenuItemClasses (Utilities|Struct|BreakS_Actors _returnvalue)))
        (CallFunction|BuildRadialItems _output_get)))))

(event Custom|TriggerAxis
  (params (MotionControllerTrans :type Transform) (AxisValue :type Float%20%28single-precision%29))
  (if (!= (Variables|Default|GetHoverIndex) -1)
    (Class|BPIMenuItems|TriggerAxis(Message) (Utilities|Array|Get(acopy) (Variables|Default|GetMenuItemActors) (Variables|Default|GetHoverIndex)) MotionControllerTrans AxisValue)))

(event Custom|TriggerActionRelease
  (if (!= (Variables|Default|GetHoverIndex) -1)
    (Class|BPIMenuItems|TriggerActionRelease(Message) (Utilities|Array|Get(acopy) (Variables|Default|GetMenuItemActors) (Variables|Default|GetHoverIndex)))))

(event Custom|Hide
  (bind _newtrack_0 (Timeline|ScaleActor Reverse)
    (:Update
      (Transformation|SetActorRelativeScale3D self (Math|Conversions|ToVector(Float) _newtrack_0)))))

(event Custom|UpdateMaterial
  (params (ThumbLocation :type Vector%202D%20Structure) (NullSelect :type Boolean) (HoverIndex :type Integer))
  (bind _returnvalue (Math|Conversions|ToFloat(Boolean) NullSelect))
  (bind _menugraphicmaterial (Variables|Default|GetMenuGraphicMaterial))
  (Rendering|Material|SetVectorParameterValue (Variables|Default|GetMenuGraphicMaterial) "ThumbLocation" (Utilities|Struct|MakeLinearColor (.x ThumbLocation) (* (.y ThumbLocation) -1.0) 0.0 1.0) :!class /Script/Engine.MaterialInstanceDynamic)
  (if NullSelect
    (Rendering|Material|SetScalarParameterValue _menugraphicmaterial "NullSelect" _returnvalue :!class /Script/Engine.MaterialInstanceDynamic)
    (else
      (Rendering|Material|SetScalarParameterValue _menugraphicmaterial "NullSelect" _returnvalue :!class /Script/Engine.MaterialInstanceDynamic)
      (Rendering|Material|SetScalarParameterValue _menugraphicmaterial "Selected" (Math|Conversions|ToFloat(Integer) HoverIndex) :!class /Script/Engine.MaterialInstanceDynamic))))

(event Custom|UnfocusMenuItem
  (if (!= (Variables|Default|GetLastHoverIndex) -1)
    (Utilities|IsValid (Utilities|Array|Get(acopy) (Variables|Default|GetMenuItemActors) (Variables|Default|GetLastHoverIndex))
      (:Is%20Valid
        (Class|BPIMenuItems|Unfocus(Message) (Utilities|Array|Get(acopy) (Variables|Default|GetMenuItemActors) (Variables|Default|GetLastHoverIndex))))
      (:Is%20Not%20Valid
        _))
    (Variables|Default|SetHoverIndex -1)
    (Variables|Default|SetLastHoverIndex -1)))

(event Custom|TriggerAction
  (params (MotionControlTrans :type Transform))
  (if (!= (Variables|Default|GetHoverIndex) -1)
    (Class|BPIMenuItems|TriggerActionPress(Message) (Utilities|Array|Get(acopy) (Variables|Default|GetMenuItemActors) (Variables|Default|GetHoverIndex)) MotionControlTrans)))

(event Custom|SelectMenuIndex
  (params (ThumbstickX :type Float%20%28single-precision%29) (ThumbstickY :type Float%20%28single-precision%29))
  (if (not (Variables|Default|GetIsHidden?))
    (CallFunction|CalcMenuIndex ThumbstickX ThumbstickY)))

(event Custom|UpdateRadialMenu
  (params (ThumbLocationX :type Float%20%28single-precision%29) (ThumbLocationY :type Float%20%28single-precision%29))
  (CallFunction|CalcMenuIndex ThumbLocationX ThumbLocationY))

(event Custom|OnSelect
  (bind _menuitemactors (Variables|Default|GetMenuItemActors))
  (bind _datatablerowhistory (Variables|Default|GetDataTableRowHistory))
  (if (!= (Variables|Default|GetHoverIndex) -1)
    (bind _returnvalue (Class|DataTableFunctionLibrary|DoesDataTableRowExist (Variables|Default|GetDataTable) (Utilities|String|StringToName (Utilities|String|LeftChop (Utilities|GetClassDisplayName (Utilities|Array|Get(acopy) (Variables|Default|GetMenuItemClasses) (Variables|Default|GetHoverIndex))) (- (Utilities|String|Len (Utilities|GetClassDisplayName (Utilities|Array|Get(acopy) (Variables|Default|GetMenuItemClasses) (Variables|Default|GetHoverIndex)))) (Utilities|String|FindSubstring (Utilities|GetClassDisplayName (Utilities|Array|Get(acopy) (Variables|Default|GetMenuItemClasses) (Variables|Default|GetHoverIndex))) "_" false true))))))
    (if _returnvalue
      (Utilities|Array|Add (Variables|Default|GetDataTableRowHistory) (Utilities|String|StringToName (Utilities|String|LeftChop (Utilities|GetClassDisplayName (Utilities|Array|Get(acopy) (Variables|Default|GetMenuItemClasses) (Variables|Default|GetHoverIndex))) (- (Utilities|String|Len (Utilities|GetClassDisplayName (Utilities|Array|Get(acopy) (Variables|Default|GetMenuItemClasses) (Variables|Default|GetHoverIndex)))) (Utilities|String|FindSubstring (Utilities|GetClassDisplayName (Utilities|Array|Get(acopy) (Variables|Default|GetMenuItemClasses) (Variables|Default|GetHoverIndex))) "_" false true)))))
      (Utilities|Array|Clear (Variables|Default|GetMenuItemClasses))
      (Variables|Default|SetHoverIndex -1)
      (Variables|Default|SetLastHoverIndex -1)
      (CallFunction|UpdateMaterial (Math|Vector2D|MakeVector2D 0.0 0.0) true)
      (CallFunction|UnfocusMenuItem)
      (for _array_element _menuitemactors
        (Class|BPIMenuItems|FadeOut(Remove)(Message) _array_element))
      (Utilities|Array|Clear _menuitemactors)
      (bind _returnvalue_2 (Utilities|GetDataTableRow (Variables|Default|GetDataTable) (Utilities|Array|Get(acopy) _datatablerowhistory (Utilities|Array|LastIndex _datatablerowhistory)))
        (:then
          (bind _output_get (Variables|Default|SetMenuItemClasses (Utilities|Struct|BreakS_Actors _returnvalue_2)))
          (CallFunction|BuildRadialItems _output_get)))
      (else
        (Development|PrintString "ROWNOTFOUND")))))

(event Custom|ShoulderSelect
  (if (!= (Variables|Default|GetHoverIndex) -1)
    (CallFunction|OnSelect)
    (Class|BPIMenuItems|Select(Message) (Utilities|Array|Get(acopy) (Variables|Default|GetMenuItemActors) (Variables|Default|GetHoverIndex)))
    (else
      (Utilities|FlowControl|FlipFlop
        (:A
          (CallFunction|Reveal)
          (Variables|Default|SetIsHidden? false))
        (:B
          (CallFunction|Hide)
          (Variables|Default|SetIsHidden? true))))))

(event EventBeginPlay
  (bind _returnvalue (Utilities|GetDataTableRow (Variables|Default|GetDataTable) (Variables|Default|GetStartingDataTableRow))
    (:then
      (bind _output_get (Variables|Default|SetMenuItemClasses (Utilities|Struct|BreakS_Actors _returnvalue)))
      (CallFunction|BuildRadialItems _output_get)
      (Utilities|Array|SetArrayElem (Variables|Default|GetDataTableRowHistory) 0 (Variables|Default|GetStartingDataTableRow) true))))

(event Collision|EventActorBeginOverlap
  (params (OtherActor :type Actor%20Object%20Reference)))

(event EventTick
  (params (DeltaSeconds :type Float%20%28single-precision%29)))

(fn ConstructionScript
  (bind _returnvalue (Rendering|Material|CreateDynamicMaterialInstance (Variables|Default|GetMenuGraphic) 0 "/RadialMenu/M_RadialLocations.M_RadialLocations" "None" :!class /Script/Engine.PrimitiveComponent))
  (bind _output_get (Variables|Default|SetMenuGraphicMaterial _returnvalue))
  (Rendering|Material|SetScalarParameterValue _output_get "InnerCircleSize" (Variables|Default|GetNullspaceSize) :!class /Script/Engine.MaterialInstanceDynamic))

(fn BuildRadialItems
  (params (MenuItems :type Array%20of%20Actor%20Class%20References))
  (bind _returnvalue (Utilities|Array|Length MenuItems))
  (Variables|Default|SetAngleBetweenItems (/ 3.6e+02 (Math|Conversions|ToFloat(Integer) _returnvalue)))
  (Rendering|Material|SetScalarParameterValue (Variables|Default|GetMenuGraphicMaterial) "Number" (Math|Conversions|ToFloat(Integer) _returnvalue) :!class /Script/Engine.MaterialInstanceDynamic)
  (for _index (range 0 (- _returnvalue 1))
    (CallFunction|AddNewItem _index)))

(fn AddNewItem
  (params (IconIndex :type Integer))
  (bind _menuradius (Variables|Default|GetMenuRadius))
  (bind _anglebetweenitems (Variables|Default|GetAngleBetweenItems))
  (bind _menuitemclasses (Variables|Default|GetMenuItemClasses))
  (bind _returnvalue (* IconIndex _anglebetweenitems))
  (bind _output (Utilities|Array|Get(acopy) _menuitemclasses IconIndex))
  (bind _returnvalue_2 (Utilities|GetClassDisplayName _output))
  (bind _returnvalue_3 (AddComponent|AddSceneComponent false (Math|Transform|MakeTransform (Math|Vector|MakeVector (+ (* (Math|Trig|Cos(Degrees) _returnvalue) _menuradius) -2.0) (* (Math|Trig|Sin(Degrees) _returnvalue) _menuradius) 0.0) "0, 0, 0" "1,1,1")))
  (bind _returnvalue_4 (Game|SpawnActorfromClass _output (Math|Transform|MakeTransform "0, 0, 0" "0, 0, 0" "1,1,1") "Undefined" 0 0))
  (Utilities|Array|SetArrayElem (Variables|Default|GetMenuItemActors) IconIndex _returnvalue_4 true)
  (Transformation|AttachComponentToComponent (Variables|/Script/Engine.Actor|GetRootComponent _returnvalue_4) _returnvalue_3 "None" "KeepRelative" "KeepRelative" "KeepRelative" false)
  (bind _returnvalue_5 (Class|DataTableFunctionLibrary|DoesDataTableRowExist (Variables|Default|GetDataTable) (Utilities|String|StringToName (Utilities|String|LeftChop _returnvalue_2 (- (Utilities|String|Len _returnvalue_2) (Utilities|String|FindSubstring _returnvalue_2 "_" false true))))))
  (if _returnvalue_5
    (bind _returnvalue_6 (AddComponent|AddStaticMeshComponent false (Math|Transform|MakeTransform "0, 0,-3.000000" "-180.000000,0.000000,0.000000" "0.300000,0.300000,0.250000")))
    (Transformation|AttachComponentToComponent _returnvalue_6 (Variables|/Script/Engine.Actor|GetRootComponent _returnvalue_4) "None" "KeepRelative" "KeepRelative" "KeepRelative" false)))

(fn CalcMenuIndex
  (params (ThumbstickX :type Float%20%28single-precision%29) (ThumbstickY :type Float%20%28single-precision%29))
  (bind _returnvalue (Class|KismetMathLibrary|VSizeXYSquared (Math|Vector|MakeVector ThumbstickX ThumbstickY 0.0)))
  (bind _menuitemclasses (Variables|Default|GetMenuItemClasses))
  (bind _returnvalue_2 (Utilities|Array|Length _menuitemclasses))
  (bind _returnvalue_3 (Class|KismetMathLibrary|DegAtan2 ThumbstickX ThumbstickY))
  (bind _returnvalue_4 (Math|Float|Sign(Float) _returnvalue_3))
  (bind _returnvalue_5 (Math|Conversions|ToFloat(Integer) _returnvalue_2))
  (bind _returnvalue_6 (- _returnvalue_4 1.0))
  (bind _returnvalue_7 (/ 3.6e+02 _returnvalue_5))
  (bind _returnvalue_8 (/ _returnvalue_6 2.0))
  (bind _returnvalue_9 (* _returnvalue_8 -3.6e+02))
  (bind _returnvalue_10 (+ _returnvalue_3 _returnvalue_9))
  (bind _returnvalue_11 (/ _returnvalue_10 _returnvalue_7))
  (bind _returnvalue_12 (Math|Float|Round _returnvalue_11))
  (bind _returnvalue_13 (Math|Integer|%(Integer) _returnvalue_12 _returnvalue_2))
  (if (!= _returnvalue 0.0)
    (if (< _returnvalue (Math|Float|Power (Variables|Default|GetNullspaceSize) 2.0))
      (Variables|Default|SetHoverIndex -1)
      (CallFunction|UpdateMaterial (Math|Vector2D|MakeVector2D ThumbstickX ThumbstickY) true)
      (CallFunction|UnfocusMenuItem)
      (else
        (if (!= (Variables|Default|GetHoverIndex) _returnvalue_13)
          (Variables|Default|SetHoverIndex _returnvalue_13)
          (CallFunction|FocusMenuItem (Variables|Default|GetHoverIndex)))
        (CallFunction|UpdateMaterial (Math|Vector2D|MakeVector2D ThumbstickX ThumbstickY) false (Variables|Default|GetHoverIndex))))))