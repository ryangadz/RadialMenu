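; BP_MenuItem is a menu item actor that displays a mesh and, on motion-controller trigger press, fires a BP_Projectile with that mesh and hue.
; The construction script applies the mesh and a dynamic material with hue shift and desaturation.
; Focus spins the mesh and plays a scale timeline, which Unfocus reverses.
; A second timeline scales it in on BeginPlay; FadeOut detaches it and reverses that timeline, destroying the actor when finished.
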(event Custom|HueShift
  (params (Shift :type Float%20%28single-precision%29)))

(event EventBeginPlay
  (Variables|Default|SetInitialTime (Utilities|Time|GetGameTimeinSeconds))
  (Default|Fadein self))

(event Collision|EventActorBeginOverlap
  (params (OtherActor :type Actor%20Object%20Reference)))

(event EventFadein
  (Variables|Default|SetInFocus? false)
  (bind (_direction _scale) (Timeline|Timeline_1 PlayFromStart)
    (:Update
      (Transformation|SetRelativeScale3D (Variables|Default|GetDefaultMeshComponent) (Math|Conversions|ToVector(Float) _scale)))
    (:Finished
      (if (Utilities|Enum|Equal(Enum) _direction (Variables|Default|GetBackward))
        (Actor|DestroyActor)))))

(event EventFadeOut(Remove)
  (Variables|Default|SetInFocus? false)
  (Transformation|DetachFromActor "KeepRelative" "KeepRelative" "KeepRelative")
  (bind (_direction _scale) (Timeline|Timeline_1 Reverse)
    (:Update
      (Transformation|SetRelativeScale3D (Variables|Default|GetDefaultMeshComponent) (Math|Conversions|ToVector(Float) _scale)))
    (:Finished
      (if (Utilities|Enum|Equal(Enum) _direction (Variables|Default|GetBackward))
        (Actor|DestroyActor)))))

(event EventTick
  (params (DeltaSeconds :type Float%20%28single-precision%29))
  (if (Variables|Default|GetInFocus?)
    (Transformation|AddRelativeRotation (Variables|Default|GetDefaultMeshComponent) (Math|Rotator|MakeRotator 0.0 0.0 (* DeltaSeconds 3.6e+02)) false false)))

(event EventFocus
  (Variables|Default|SetInFocus? true)
  (bind (_direction _scale _saturation) (Timeline|Timeline_0 PlayFromStart)
    (:Update
      (Transformation|SetRelativeScale3D (Variables|Default|GetDefaultMeshComponent) (Math|Conversions|ToVector(Float) _scale)))))

(event EventUnfocus
  (Variables|Default|SetInFocus? false)
  (bind (_direction _scale _saturation) (Timeline|Timeline_0 Reverse)
    (:Update
      (Transformation|SetRelativeScale3D (Variables|Default|GetDefaultMeshComponent) (Math|Conversions|ToVector(Float) _scale)))))

(event EventRemove)

(event EventTriggerActionPress
  (params (MotionControlTrans :type Transform))
  (Game|SpawnActorfromClass "/RadialMenu/BP_Projectile.BP_Projectile_C" MotionControlTrans "Undefined" 0 (Variables|/Script/Engine.StaticMeshComponent|GetStaticMesh (Variables|Default|GetDefaultMeshComponent)) 15.0 (Variables|Default|GetColorHueShift) 0))

(fn ConstructionScript
  (bind _defaultmeshcomponent (Variables|Default|GetDefaultMeshComponent))
  (Components|StaticMesh|SetStaticMesh _defaultmeshcomponent (Variables|Default|GetStaticMesh))
  (bind _returnvalue (Rendering|Material|CreateDynamicMaterialInstance _defaultmeshcomponent 0 (Variables|Default|GetParentMaterial) "None" :!class /Script/Engine.PrimitiveComponent))
  (bind _output_get (Variables|Default|SetDynamicMaterial _returnvalue))
  (Rendering|Material|SetScalarParameterValue _output_get "Desaturation" (- 1.0 (Variables|Default|GetSaturation)) :!class /Script/Engine.MaterialInstanceDynamic)
  (Rendering|Material|SetScalarParameterValue (Variables|Default|GetDynamicMaterial) "HueShift" (Variables|Default|GetColorHueShift) :!class /Script/Engine.MaterialInstanceDynamic))